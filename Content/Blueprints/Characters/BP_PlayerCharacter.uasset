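; Player character Blueprint that handles variable-height jump input and a left-mouse attack state.
; Jumping starts only when grounded, at normal gravity; releasing the key, or still holding it after a short delay, stops the jump and raises gravity for a faster fall.
; It maintains Jumping, Falling and AttackStarted flags, with the attack flag clearing on a delay after mouse release.
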(event `InputAction|Jump`
  (params (Key :type "Key Structure"))
  (:`Pressed`
    (set `self.Jumping` true)
    (if (not (`NavMovementComponent.IsFalling` (`self.CharacterMovement`)))
      (set `self.Falling` false)
      (if (`self.Falling`) :!label _label
        (set `CharacterMovementComponent.GravityScale` 3.0 (`self.CharacterMovement`))
        (`self.StopJumping`)
        (set `self.Jumping` false)
        (else
          (set `CharacterMovementComponent.GravityScale` 1.0 (`self.CharacterMovement`))
          (`self.Jump`)
          (`KismetSystemLibrary.Delay` 0.5)
          (if (`PlayerController.IsInputKeyDown` (`GameplayStatics.GetPlayerController` 0) Key)
            (set `CharacterMovementComponent.GravityScale` 3.0 (`self.CharacterMovement`))
            (`self.StopJumping`)
            (`KismetSystemLibrary.Delay` 0.2)
            (set `self.Jumping` false))))))
  (:`Released`
    (set `self.Falling` true)
    (goto _label)))

(event `Key|LeftMouseButton`
  (params (Key :type "Key Structure"))
  (:`Pressed`
    (set `self.AttackStarted` true))
  (:`Released`
    (`KismetSystemLibrary.Delay` 1.3)
    (set `self.AttackStarted` false)))

(fn `UserConstructionScript`)