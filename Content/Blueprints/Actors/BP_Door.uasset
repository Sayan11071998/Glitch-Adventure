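; BP_Door is a level-exit door that shows the player a HUD prompt based on whether they carry a key.
; Two seconds after BeginPlay, it caches the HUD widget reference from BP_GlitchAdventure_GameMode.
; Player overlap checks HasKey and calls DoorKeyInfo with either a finish-level or key-needed message, and leaving deactivates it.
; The Enter input and level completion are not handled in this Blueprint.
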(event `self.ReceiveBeginPlay`
  (`KismetSystemLibrary.Delay` 2.0)
  (bind _asbp_glitch_adventure_game_mode (cast `/Game/Blueprints/BP_GlitchAdventure_GameMode` (`GameplayStatics.GetGameMode`)))
  (set `self.UI_HUD_REF` (`/Game/Blueprints/BP_GlitchAdventure_GameMode.UI_HUD_REF` _asbp_glitch_adventure_game_mode)))

(event `self.ReceiveActorBeginOverlap`
  (params (OtherActor :type "Actor Object Reference"))
  (bind _ui_hud_ref (`self.UI_HUD_REF`))
  (bind _asbp_player_character (cast `/Game/Blueprints/Characters/BP_PlayerCharacter` OtherActor))
  (if (`PlayerCharacter.HasKey` _asbp_player_character)
    (`/Game/Blueprints/Widgets/WBP_UI_HUD.DoorKeyInfo` _ui_hud_ref "Press \"Enter\" To Finish The Level" true)
    (else
      (`/Game/Blueprints/Widgets/WBP_UI_HUD.DoorKeyInfo` _ui_hud_ref "You Need A Key To Open This Door" true))))

(event `self.ReceiveActorEndOverlap`
  (params (OtherActor :type "Actor Object Reference"))
  (cast `/Game/Blueprints/Characters/BP_PlayerCharacter` OtherActor)
  (`/Game/Blueprints/Widgets/WBP_UI_HUD.DoorKeyInfo` (`self.UI_HUD_REF`) "You Need A Key To Open This Door" false))

(fn `UserConstructionScript`)